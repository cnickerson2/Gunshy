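; Game mode for the turtle tile pattern in Gunshy, which lays out the tiles when play begins.
; BeginPlay calls the parent, initializes the tile pool, then places the tiles.
; The layout is defined by components under DefaultSceneRoot: each descendant marks a position, and a tile checked out of the pool is teleported to its world location.
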(event `self.ReceiveBeginPlay`
  (`parent.ReceiveBeginPlay`)
  (`self.InitializePool`)
  (`self.Place Tiles`))

(fn `Place Tiles`
  (for _array_element (`SceneComponent.GetChildrenComponents` (`self.DefaultSceneRoot`) true)
    (bind _returnvalue (`TilePool.Checkout` (`self.TilePool`)))
    (`self.K2_SetActorLocation` _returnvalue (`SceneComponent.K2_GetComponentLocation` _array_element) false true)))

(fn `UserConstructionScript`
  (`parent.UserConstructionScript`))